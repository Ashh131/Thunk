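; Shared multiplayer camera actor that stays centred on all players and zooms to keep them on screen.
; Each Tick it moves to the average location of the player pawns, using the game mode's player count and pawn indices.
; It then maps the farthest pawn's distance from that centre through a clamped zoom range, scaled by MinArmLength, to set the spring arm length.
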(event `self.ReceiveTick`
  (params (DeltaSeconds :type "Float (single-precision)"))
  ; Camera Control - Makes the camera always in the centre of all the players and makes sure they all stay on screen
  (bind _returnvalue (`GameModeBase.GetNumPlayers` (`GameplayStatics.GetGameMode`)))
  (set `self.LocationSum` (0.0 0.0 0.0))
  (for _index (range _returnvalue)
    (set `self.LocationSum` (+ (`self.LocationSum`) (`self.K2_GetActorLocation` (`GameplayStatics.GetPlayerPawn` _index)))))
  (`self.K2_SetActorLocation` (/ (`self.LocationSum`) _returnvalue))
  (set `self.BiggestFromCenter` 0.0)
  (bind _returnvalue_2 (`GameModeBase.GetNumPlayers` (`GameplayStatics.GetGameMode`)))
  (for _index_2 (range _returnvalue_2)
    (bind _returnvalue_3 (`KismetMathLibrary.Vector_Distance` (`self.K2_GetActorLocation`) (`self.K2_GetActorLocation` (`GameplayStatics.GetPlayerPawn` _index_2))))
    (if (> _returnvalue_3 (`self.BiggestFromCenter`))
      (set `self.BiggestFromCenter` _returnvalue_3)))
  (set `SpringArmComponent.TargetArmLength` (* (`KismetMathLibrary.MapRangeClamped` (`self.BiggestFromCenter`) (`self.MinFromCenter`) (`self.MaxFromCenter`) (`self.MinZoom`) (`self.MaxZoom`)) (`self.MinArmLength`)) (`self.SpringArm`)))

(fn `UserConstructionScript`)